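; BP_BaseBuildingType3 is a building subclass that accumulates a portal resource counter.
; Each transmitter widget update runs the parent logic, increments PortalResource, refreshes the count through UpdateResCount, and writes it to the LevelSaveObject on FirstPersonGameMode.
; BeginPlay shows the current count, while Init, construction and source widget updates only defer to the parent.
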(event EventInit
  (|CallParentFunction))

(event EventBeginPlay
  (CallFunction|UpdateResCount (Variables|Default|GetPortalResource)))

(fn ConstructionScript
  (|CallParentFunction))

(fn UpdateTransmitterBuildingWidget
  (|CallParentFunction)
  (bind _output_get (Variables|Default|SetPortalResource (+ (Variables|Default|GetPortalResource) 1)))
  (CallFunction|UpdateResCount _output_get)
  (bind _asfirst_person_game_mode (Utilities|Casting|CastToFirstPersonGameMode (Game|GetGameMode)))
  (Variables|/Game/Game/Blueprints/SaveGame/S_LevelDataObject.S_LevelDataObject_C|SetPortalResource (Variables|/Game/Game/Blueprints/FirstPersonGameMode.FirstPersonGameMode_C|GetLevelSaveObject _asfirst_person_game_mode) (Variables|Default|GetPortalResource)))

(fn UpdateSourceBuildingWidget
  (params (BaseBuilding :type BP%20Base%20Building%20Object%20Reference))
  (|CallParentFunction BaseBuilding))