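; BP_BaseBuilding is a base building actor that shows an info widget with a resource count.
; On BeginPlay it passes SourceResource to the WBP_BuildingInfo widget as its count.
; A Box trigger shows the widget component while the player pawn overlaps it and hides it on exit.
; It also exposes an arrow visibility toggle and a placeholder FindNearestActorofClass that just returns self.
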(event OnComponentBeginOverlap(Box)
  (params (OverlappedComponent :type Primitive%20Component%20Object%20Reference) (OtherActor :type Actor%20Object%20Reference) (OtherComp :type Primitive%20Component%20Object%20Reference) (OtherBodyIndex :type Integer) (bFromSweep :type Boolean) (SweepResult :type Hit%20Result%20Structure%20%28by%20ref%29))
  (if (== OtherActor (Game|Player|GetPlayerPawn 0))
    (CallFunction|SetVisibility3DWidget true)))

(event OnComponentEndOverlap(Box)
  (params (OverlappedComponent :type Primitive%20Component%20Object%20Reference) (OtherActor :type Actor%20Object%20Reference) (OtherComp :type Primitive%20Component%20Object%20Reference) (OtherBodyIndex :type Integer))
  (if (== OtherActor (Game|Player|GetPlayerPawn 0))
    (CallFunction|SetVisibility3DWidget false)))

(event EventBeginPlay
  (CallFunction|UpdateResCount (Variables|Default|GetSourceResource)))

(fn ConstructionScript)

(fn UpdateResCount
  (params (InText :type Integer))
  (bind _aswbp_building_info (Utilities|Casting|CastToWBP_BuildingInfo (UserInterface|GetWidget (Variables|Default|GetWidget))))
  (Variables|/Game/Game/Blueprints/Buildings/WBP_BuildingInfo.WBP_BuildingInfo_C|SetCount _aswbp_building_info InText)
  (Default|SetText _aswbp_building_info))

(fn FindNearestActorofClass
  (params (Class :type Actor%20Class%20Reference) (TargetLocation :type Vector :default "0, 0, 0"))
  (return (Utilities|ResolveSoftReference self)))

(fn SetVisibility3DWidget
  (params (bNewVisibility :type Boolean))
  (Rendering|SetVisibility (Variables|Default|GetWidget) bNewVisibility false))

(fn SetVisibilityArrow
  (params (bNewVisibility :type Boolean))
  (Rendering|SetVisibility (Variables|Default|GetArrow) bNewVisibility false))