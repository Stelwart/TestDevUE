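; Transmitter building Blueprint that pulls resources from the nearest BP_BaseBuilding over time.
; A looping timer started on Init moves one unit per tick, updating both buildings' counters and aiming an arrow at the source.
; Its own SourceResource mirrors the collected amount or the saved PortalResource, depending on BuildingType.
; Collection stops when the source empties or the transmitter passes its cap; SavePortalResource is never called here.
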(event Custom|Collect
  (bind _nearest_actor (CallFunction|FindNearestActorOfClass "/Game/Game/Blueprints/Buildings/BP_BaseBuilding.BP_BaseBuilding_C" (Transformation|GetActorLocation self)))
  (bind _object (Utilities|AsyncLoadAsset _nearest_actor)
    (:Completed
      (bind _asbp_base_building (Utilities|Casting|CastToBP_BaseBuilding _object))
      (if (<= (Variables|Default|GetTransmitterResource) 100)
        (if (> (Variables|/Game/Game/Blueprints/Buildings/BP_BaseBuilding.BP_BaseBuilding_C|GetSourceResource _asbp_base_building) 0)
          (CallFunction|UpdateTransmitterBuildingWidget)
          (CallFunction|UpdateSourceBuildingWidget _asbp_base_building)
          (Utilities|FlowControl|Sequence
            (:then_0
              ;[1 1 1] Updating Source resource
              (switch Utilities|FlowControl|Switch|SwitchonE_BuildingType (Variables|Default|GetBuilding%20Type)
                (:NewEnumerator1
                  (Variables|Default|SetSourceResource (Variables|Default|GetTransmitterResource)))
                (:NewEnumerator2
                  (bind _asfirst_person_game_mode (Utilities|Casting|CastToFirstPersonGameMode (Game|GetGameMode)))
                  (Variables|Default|SetSourceResource (Variables|/Game/Game/Blueprints/SaveGame/S_LevelDataObject.S_LevelDataObject_C|GetPortalResource (Variables|/Game/Game/Blueprints/FirstPersonGameMode.FirstPersonGameMode_C|GetLevelSaveObject _asfirst_person_game_mode))))))
            (:then_1
              ;[1 1 1] Arrow logic
              (CallFunction|SetVisibilityArrow true)
              (Transformation|SetRelativeRotation (Variables|Default|GetArrow) (Math|Rotator|MakeRotator 0.0 0.0 (.yaw (Math|Rotator|FindLookatRotation (Transformation|GetActorLocation self) (Transformation|GetActorLocation _asbp_base_building)))) false false)))
          (else
            ;[1 1 1] Stopping the collect
            (Utilities|Time|ClearandInvalidateTimerbyHandle (Variables|Default|GetTimerHandle) :!label _label)
            (CallFunction|SetVisibilityArrow false)))
        (else
          (goto _label))))))

(event Custom|Init
  (bind _returnvalue (Utilities|Time|SetTimerbyEvent (delegate Custom|Collect) 1.0 true))
  (Variables|Default|SetTimerHandle _returnvalue))

(fn ConstructionScript
  (|CallParentFunction))

(fn UpdateTransmitterBuildingWidget
  (bind _output_get (Variables|Default|SetTransmitterResource (+ (Variables|Default|GetTransmitterResource) 1)))
  (CallFunction|UpdateResCount _output_get))

(fn UpdateSourceBuildingWidget
  (params (BaseBuilding :type BP%20Base%20Building%20Object%20Reference))
  (bind _output_get (Variables|Default|SetSourceResource BaseBuilding (- (Variables|/Game/Game/Blueprints/Buildings/BP_BaseBuilding.BP_BaseBuilding_C|GetSourceResource BaseBuilding) 1)))
  (Default|UpdateResCount BaseBuilding _output_get))

(fn SavePortalResource
  (switch Utilities|FlowControl|Switch|SwitchonE_BuildingType (Variables|Default|GetBuilding%20Type)
    (:NewEnumerator2
      (bind _asfirst_person_game_mode (Utilities|Casting|CastToFirstPersonGameMode (Game|GetGameMode)))
      (Variables|/Game/Game/Blueprints/SaveGame/S_LevelDataObject.S_LevelDataObject_C|SetPortalResource (Variables|/Game/Game/Blueprints/FirstPersonGameMode.FirstPersonGameMode_C|GetLevelSaveObject _asfirst_person_game_mode) (Variables|Default|GetTransmitterResource)))))